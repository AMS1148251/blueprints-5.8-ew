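; Collectable pickup actor that awards an amount to the third-person player character when touched.
; A box overlap casts the other actor to BP_ThirdPersonCharacter, calls CollectPickup with its increase amount, then destroys itself.
; The sphere mesh gets one material in the construction script and a different one at BeginPlay, with debug prints of its location and failed overlaps.
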(event `self.ReceiveBeginPlay`
  (`KismetSystemLibrary.PrintString` (`KismetStringLibrary.Conv_VectorToString` (`SceneComponent.K2_GetComponentLocation` (`self.Sphere`))) true true (struct :`R` 1.0 :`B` 0.053151 :`A` 1.0) 10.0)
  (`PrimitiveComponent.SetMaterial` (`self.Sphere`) 0 "/Engine/MapTemplates/Materials/BasicAsset03.BasicAsset03"))

(event `self.Box.OnComponentBeginOverlap`
  (params (OverlappedComponent :type "PrimitiveComponent Object Reference") (OtherActor :type "Actor Object Reference") (OtherComp :type "PrimitiveComponent Object Reference") (OtherBodyIndex :type Integer) (bFromSweep :type Boolean) (SweepResult :type "HitResult Structure (by ref)"))
  ; check if collied by plr
  (bind _asbp_third_person_character (cast `/Game/ThirdPerson/Blueprints/BP_ThirdPersonCharacter` OtherActor)
    (:`then`
      (`/Game/ThirdPerson/Blueprints/BP_ThirdPersonCharacter.collect pickup` _asbp_third_person_character (`self.Increaced Aount`))
      (`self.K2_DestroyActor`))
    (:`CastFailed`
      _))
  (`KismetSystemLibrary.PrintString` (`KismetSystemLibrary.GetDisplayName` OtherActor)))

(fn `UserConstructionScript`
  (`PrimitiveComponent.SetMaterial` (`self.Sphere`) 0 "/Engine/EngineDebugMaterials/BoneWeightMaterial.BoneWeightMaterial"))