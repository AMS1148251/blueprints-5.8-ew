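; Goal trigger that checks whether the third-person character has collected enough balls when it overlaps the box.
; At or above NeedBalls, it prints a success message and plays a click sound, with no further progression.
; Below that, it prints a death message, spawns particles and sound at the box, destroys the character, then after a short delay calls OpenLevel with the level name left as None.
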(event `self.Box.OnComponentBeginOverlap`
  (params (OverlappedComponent :type "PrimitiveComponent Object Reference") (OtherActor :type "Actor Object Reference") (OtherComp :type "PrimitiveComponent Object Reference") (OtherBodyIndex :type Integer) (bFromSweep :type Boolean) (SweepResult :type "HitResult Structure (by ref)"))
  (bind _returnvalue (`SceneComponent.K2_GetComponentLocation` (`self.Box`)))
  (bind _asbp_third_person_character (cast `/Game/ThirdPerson/Blueprints/BP_ThirdPersonCharacter` OtherActor))
  (if (>= (`/Game/ThirdPerson/Blueprints/BP_ThirdPersonCharacter.collected amount` _asbp_third_person_character) (`self.need balls`))
    (`KismetSystemLibrary.PrintString` (`KismetStringLibrary.Concat_StrStr` "u got balls" (`KismetStringLibrary.Conv_IntToString` (`self.need balls`))))
    (`GameplayStatics.PlaySound2D` "/Engine/VREditor/Sounds/VR_click2.VR_click2" 1.0 1.0 0.0 null null)
    (else
      (`KismetSystemLibrary.PrintString` "u died")
      (`GameplayStatics.SpawnEmitterAtLocation` "/Engine/Tutorial/SubEditors/TutorialAssets/TutorialParticleSystem.TutorialParticleSystem" _returnvalue)
      (`GameplayStatics.PlaySoundAtLocation` "/Engine/EditorSounds/GamePreview/EndPlayInEditor.EndPlayInEditor" _returnvalue (struct) 1.0 1.0 0.0 null null null null)
      (`self.K2_DestroyActor` _asbp_third_person_character)
      (`KismetSystemLibrary.Delay` 2.0)
      (`GameplayStatics.OpenLevel` "None"))))

(fn `UserConstructionScript`)