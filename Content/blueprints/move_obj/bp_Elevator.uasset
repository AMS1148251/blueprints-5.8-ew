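; Elevator Blueprint that moves a Cube back and forth between the Bottompos and Toppos components, starting at BeginPlay.
; A FlipFlop in the RepertMove event alternates the MovePlr timeline between playing from start and reversing from end.
; The timeline's alpha lerps the Cube's world location without sweep, and its Finished output calls RepertMove again to repeat the motion.
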(event `self.ReceiveBeginPlay`
  (`self.repert move`))

(event `repert move`
  (`/Engine/EditorBlueprintResources/StandardMacros.FlipFlop`
    (:`A`
      (bind (_direction _alfha) (`Timeline|move plr` :!via `PlayFromStart` :!label _label)
        (:`Update`
          (`SceneComponent.K2_SetWorldLocation` (`self.Cube`) (`KismetMathLibrary.VLerp` (`SceneComponent.K2_GetComponentLocation` (`self.bottompos`)) (`SceneComponent.K2_GetComponentLocation` (`self.toppos`)) _alfha) false false))
        (:`Finished`
          (`self.repert move`))))
    (:`B`
      (goto _label :!via `ReverseFromEnd`))))

(fn `UserConstructionScript`)